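; Campfire actor whose particle effect scales over time when Q is pressed, with input enabled while a ThirdPersonCharacter overlaps its box.
; Two Q handlers restart timelines: one drives the particle system's scale, the other updates and prints CampfireParameter.
; Overlap also toggles Addfire, but the logic gating fire on Havingwood and Addfire is disconnected and never runs.
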(event `self.Box.OnComponentBeginOverlap`
  (params (OverlappedComponent :type "PrimitiveComponent Object Reference") (OtherActor :type "Actor Object Reference") (OtherComp :type "PrimitiveComponent Object Reference") (OtherBodyIndex :type Integer) (bFromSweep :type Boolean) (SweepResult :type "HitResult Structure (by ref)"))
  (cast `/Game/ThirdPersonBP/Blueprints/ThirdPersonCharacter` OtherActor)
  (`self.EnableInput` (`GameplayStatics.GetPlayerController` 0))
  (`KismetSystemLibrary.PrintString` "Hello")
  (set `self.Addfire` true))

(event `self.Box.OnComponentEndOverlap`
  (params (OverlappedComponent :type "PrimitiveComponent Object Reference") (OtherActor :type "Actor Object Reference") (OtherComp :type "PrimitiveComponent Object Reference") (OtherBodyIndex :type Integer))
  (cast `/Game/ThirdPersonBP/Blueprints/ThirdPersonCharacter` OtherActor)
  (`self.DisableInput` (`GameplayStatics.GetPlayerController` 0))
  (set `self.Addfire` false))

(event `Key|Q`
  (params (Key :type "Key Structure"))
  (:`Pressed`
    (bind (_direction _newtrack_0) (`Timeline|Timeline_0` :!via `PlayFromStart`)
      (:`Update`
        (`SceneComponent.SetWorldScale3D` (`self.ParticleSystem`) (`KismetMathLibrary.Conv_DoubleToVector` _newtrack_0))))))

(event `Key|Q`
  (params (Key :type "Key Structure"))
  (:`Pressed`
    (bind (_direction _newtrack_0) (`Timeline|Timeline_1` :`NewTime` (`self.campfire_parameter`) :!via `PlayFromStart`)
      (:`Update`
        (bind _output_get (set `self.campfire_parameter` _newtrack_0))
        (`KismetSystemLibrary.PrintString` (`KismetStringLibrary.Conv_DoubleToString` _output_get))))))

(fn `UserConstructionScript`)