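; Clover is a physics prop tied to the player's holding state that destroys itself on overlapping Lucy, clearing that holding flag.
; Each tick reads the player character's Isholding flag, lowering mesh linear damping and hiding the prompt widget while held, otherwise applying heavy damping to resist movement.
; A box overlap sets CanInteract and shows or hides the widget for the player.
; A looping timer resets the widget's world rotation to zero.
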(event `self.ReceiveActorBeginOverlap`
  (params (OtherActor :type "Actor Object Reference"))
  (cast `/Game/Content/Blueprints/Lucy` OtherActor)
  (`self.K2_DestroyActor`)
  (set `/Game/ThirdPersonBP/Blueprints/ThirdPersonCharacter.isholding` false (`self.As Third Person Character_1`)))

(event `self.ReceiveTick`
  (params (DeltaSeconds :type "Float (single-precision)"))
  (bind _staticmesh (`self.StaticMesh`))
  (if (`/Game/ThirdPersonBP/Blueprints/ThirdPersonCharacter.isholding` (`self.As Third Person Character_1`))
    (`PrimitiveComponent.SetLinearDamping` _staticmesh 0.1)
    (`SceneComponent.SetVisibility` (`self.Widget`) false false)
    (else
      (`PrimitiveComponent.SetLinearDamping` _staticmesh 500.0))))

(event `self.ReceiveBeginPlay`
  (`|ExecutionSequence`
    (:`then_0`
      (`self.Player Cast`))
    (:`then_1`
      (`self.Widget Detection`))))

(event `Player Cast`
  (bind _asthird_person_character (cast `/Game/ThirdPersonBP/Blueprints/ThirdPersonCharacter` (`GameplayStatics.GetPlayerCharacter` 0)))
  (set `self.As Third Person Character_1` _asthird_person_character))

(event `Widget Detection`
  ;[1 1 1] Widget Detection
  (`|ExecutionSequence`
    (:`then_0`
      (bind _asthird_person_character (cast `/Game/ThirdPersonBP/Blueprints/ThirdPersonCharacter` (`GameplayStatics.GetPlayerCharacter` 0)))
      (set `self.As Third Person Character_1` _asthird_person_character)
      (`SceneComponent.SetVisibility` (`self.Widget`) false false))
    (:`then_1`
      (`KismetSystemLibrary.K2_SetTimerDelegate` (delegate `Spin`) 0.1 true))))

(event `Spin`
  ;[1 1 1] Widget Detection
  (`SceneComponent.K2_SetWorldRotation` (`self.Widget`) (`KismetMathLibrary.MakeRotator` 0.0) false false))

(event `self.Box.OnComponentBeginOverlap`
  (params (OverlappedComponent :type "PrimitiveComponent Object Reference") (OtherActor :type "Actor Object Reference") (OtherComp :type "PrimitiveComponent Object Reference") (OtherBodyIndex :type Integer) (bFromSweep :type Boolean) (SweepResult :type "HitResult Structure (by ref)"))
  ;[1 1 1] Widget Detection
  (if (== OtherActor (`self.As Third Person Character_1`))
    (set `self.Can Interact` true)
    (`SceneComponent.SetVisibility` (`self.Widget`) true false)))

(event `self.Box.OnComponentEndOverlap`
  (params (OverlappedComponent :type "PrimitiveComponent Object Reference") (OtherActor :type "Actor Object Reference") (OtherComp :type "PrimitiveComponent Object Reference") (OtherBodyIndex :type Integer))
  ;[1 1 1] Widget Detection
  (if (== (`self.As Third Person Character_1`) OtherActor)
    (set `self.Can Interact` false)
    (`SceneComponent.SetVisibility` (`self.Widget`) false false)))

(fn `UserConstructionScript`)