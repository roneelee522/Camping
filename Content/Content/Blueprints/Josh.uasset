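; Josh is a Blueprint with a capsule that reacts to overlapping pinecones and tracks a friendship score for a task.
; Each Pinecone_bp overlap raises FriendshipJosh by one, shows the Josh_progression widget and pauses the game.
; When the next increment would reach the target of ten, it shows Josh_taskcomplete instead, without storing the increment or pausing.
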(event `self.CapsuleComponent.OnComponentBeginOverlap`
  (params (OverlappedComponent :type "PrimitiveComponent Object Reference") (OtherActor :type "Actor Object Reference") (OtherComp :type "PrimitiveComponent Object Reference") (OtherBodyIndex :type Integer) (bFromSweep :type Boolean) (SweepResult :type "HitResult Structure (by ref)"))
  (bind _returnvalue (+ (`self.friendship_Josh`) 1.0))
  (cast `/Game/Content/Blueprints/Pinecone_bp` OtherActor)
  (if (== _returnvalue 10.0)
    (bind _returnvalue_2 (`|CreateWidget` "/Game/UI/Josh_taskcomplete.Josh_taskcomplete_C"))
    (`UserWidget.AddToViewport` _returnvalue_2 0)
    (else
      (set `self.friendship_Josh` _returnvalue)
      (bind _returnvalue_3 (`|CreateWidget` "/Game/UI/Josh_progression.Josh_progression_C"))
      (`UserWidget.AddToViewport` _returnvalue_3 0)
      (`GameplayStatics.SetGamePaused` true))))

(fn `UserConstructionScript`)